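; GMBase is the game mode of a pinball game, running the menu, lives, score and currency across runs.
; On BeginPlay it shows the main menu widget with its upgrade menu, whose BonusLife adds to the starting lives.
; Balls spawn through the Flipper_1 pawn, which also displays bumper score; each lost ball costs a life.
; Game over converts half the score into currency, sets the high score and reshows the menu.
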(event `self.ReceiveBeginPlay`
  ; Lancement du menu
  (set `PlayerController.bShowMouseCursor` true (`GameplayStatics.GetPlayerController` 0))
  (bind _returnvalue (`|CreateWidget` "/Game/MenuSystem/WB_MainMenuUi.WB_MainMenuUi_C"))
  (bind _output_get (set `self.MenuUI` _returnvalue))
  (`UserWidget.AddToViewport` _output_get 0)
  (`/Game/MenuSystem/WB_MainMenuUi.CreateUpgradeMenu` (`self.MenuUI`)))

(event `spawnNewBall`
  ; Spawn new ball
  (bind _asflipper_1 (cast `/Game/Blueprints/Pawns/Flipper_1` (`GameplayStatics.GetPlayerPawn` 0)))
  (`/Game/Blueprints/Pawns/Flipper_1.SpawnBall` _asflipper_1))

(event `StartGame`
  ; Lancement de la game
  (set `self.CurrentLife` (+ (`/Game/MenuSystem/WB_UpgradeMenu.Bonus_Life` (`/Game/MenuSystem/WB_MainMenuUi.MenuUpgrade` (`self.MenuUI`))) 2))
  (set `self.GameCurrentScore` 0)
  (`self.spawnNewBall`))

(event `AddMonnaie`
  (params (Monnaie :type Integer64))
  ; Ajoute le montant de monnaie au compte
  (bind _output_get (set `self.CurrentMonnaie` (+ Monnaie (`self.CurrentMonnaie`))))
  (`/Game/MenuSystem/WB_MainMenuUi.UpdateMonnaie` (`self.MenuUI`) _output_get))

(event `BallOut`
  ; Quand la balle sort
  (bind _output_get (set `self.CurrentLife` (- (`self.CurrentLife`) 1)))
  (if (> _output_get 0)
    (`self.spawnNewBall`)
    (else
      (`self.GameOver`))))

(event `ScoreToMonnaie`
  (params (Score :type Integer64))
  ; Divise le score / 2 = monnaie gagnée
  (`self.AddMonnaie` (/ Score 2)))

(event `AddBumperScore`
  ; Ajoute le score du bumper au score actuel
  (bind _output_get (set `self.GameCurrentScore` (+ (`self.GameCurrentScore`) (`self.CurrentBumperScore`))))
  (bind _asflipper_1 (cast `/Game/Blueprints/Pawns/Flipper_1` (`GameplayStatics.GetPlayerPawn` 0)))
  (`/Game/Blueprints/Pawns/Flipper_1.UpdateScore` _asflipper_1 _output_get))

(event `GameOver`
  ; En cas de game over
  (`self.ScoreToMonnaie` (`self.GameCurrentScore`))
  (`/Game/MenuSystem/WB_MainMenuUi.SetHighScore` (`self.MenuUI`) (`self.GameCurrentScore`))
  (`Widget.SetVisibility` (`self.MenuUI`) "Visible"))

(fn `UserConstructionScript`)