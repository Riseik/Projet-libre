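; BP_Bumper is a pinball-style bumper actor that knocks the ball away on contact and awards points.
; When a BP_BallFlipper overlaps its Sphere, it applies an impulse to that actor's StaticMesh, directed outward from the Center component and scaled by Force.
; It then plays a hit sound at Center and calls AddBumperScore on the GMBase game mode.
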(event `self.Sphere.OnComponentBeginOverlap`
  (params (OverlappedComponent :type "PrimitiveComponent Object Reference") (OtherActor :type "Actor Object Reference") (OtherComp :type "PrimitiveComponent Object Reference") (OtherBodyIndex :type Integer) (bFromSweep :type Boolean) (SweepResult :type "HitResult Structure (by ref)"))
  (bind _returnvalue (`SceneComponent.K2_GetComponentLocation` (`self.Center`)))
  (bind _asbp_ball_flipper (cast `/Game/Blueprints/Actor/BP_BallFlipper` OtherActor))
  (`PrimitiveComponent.AddImpulse` (`/Game/Blueprints/Actor/BP_BallFlipper.StaticMesh` _asbp_ball_flipper) (* (`KismetMathLibrary.Normal` (- (`self.K2_GetActorLocation` _asbp_ball_flipper) _returnvalue)) (`self.Force`)) "None" false)
  (`GameplayStatics.PlaySoundAtLocation` "/Game/Sound/SND_BumperHit.SND_BumperHit" _returnvalue (struct) 1.0 1.0 0.0 null null null null)
  (bind _asgmbase (cast `/Game/Blueprints/GameModes/GMBase` (`GameplayStatics.GetGameMode`)))
  (`/Game/Blueprints/GameModes/GMBase.AddBumperScore` _asgmbase))

(fn `UserConstructionScript`)